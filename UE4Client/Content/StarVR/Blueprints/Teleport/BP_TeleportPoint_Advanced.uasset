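; BP_TeleportPoint_Advanced is a VR teleport skill actor that shows a target ring and glides the character to the chosen point.
; Activating or deactivating the skill toggles visibility, while placement moves the ring and tints its dynamic material blue or red by validity.
; Casting stores start, end and mesh offset through server/multicast-named events, then a timeline lerps the character's location.
; The move triggers the teleport effect and switches animation to FK-only, restoring IK shortly after arrival.
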(event Custom|TeleportEndMulticast
  (bind _chracteractor (Variables|Default|GetChracterActor))
  ;[1 1 1] 服务器执行传送过程
  (Class|BPIPlayerPawn|ActiveTeleportEffect(Message) _chracteractor)
  (bind _animinstance (Class|BPIPlayerPawn|GetChrAnimInstance(Message) _chracteractor))
  (Class|BPICharacterAction|OnlyDoFKAnim(Message) _animinstance "NewEnumerator0")
  (bind _lerp (Timeline|Timeline_0 PlayFromStart)
    (:Update
      (Transformation|SetActorLocation _chracteractor (- (Math|Vector|Lerp(Vector) (Variables|Default|GetTeleportStartPosServer) (Variables|Default|GetTeleportEndPosServer) _lerp) (Variables|Default|GetTeleportMeshOffset)) false false))
    (:Finished
      (bind _animinstance_2 (Class|BPIPlayerPawn|GetChrAnimInstance(Message) (Variables|Default|GetChracterActor)))
      (Class|BPICharacterAction|OnlyDoFKAnim(Message) _animinstance_2 "NewEnumerator1")
      (Utilities|FlowControl|Delay 0.2)
      (bind _animinstance_3 (Class|BPIPlayerPawn|GetChrAnimInstance(Message) (Variables|Default|GetChracterActor)))
      (Class|BPICharacterAction|UseIKAnim(Message) _animinstance_3))))

(event Custom|SetTeleportParaSvr
  (params (StartPos :type Vector) (EndPos :type Vector) (MeshOffset :type Vector))
  (Variables|Default|SetTeleportStartPosServer StartPos)
  (Variables|Default|SetTeleportEndPosServer EndPos)
  (Variables|Default|SetTeleportMeshOffset MeshOffset)
  (CallFunction|TeleportEndMulticast))

(event Custom|ShowRingMuilticast
  (params (EndPos :type Vector) (ValidatePos :type Boolean))
  (bind _dmi_targetcurcle (Variables|Default|GetDMI_TargetCurcle))
  ;[1 1 1] 设置指示位置
  (Utilities|IsValid _dmi_targetcurcle
    (:Is%20Valid
      (Rendering|Material|SetVectorParameterValue _dmi_targetcurcle "EmissiveColor" (select ValidatePos "(R=0.200000,G=0.400000,B=1.000000,A=1.000000)" "(R=1.000000,G=0.000000,B=0.043773,A=1.000000)") :!class /Script/Engine.MaterialInstanceDynamic))
    (:Is%20Not%20Valid
      _))
  (Transformation|SetWorldLocationAndRotation (Variables|Default|GetTeleportTargetCircle) EndPos "0.000000, 0, 0" false false))

(event EventCastSkill
  (params (StartPos :type Vector) (EndPos :type Vector) (MeshOffset :type Vector))
  ;[1 1 1] Set Offset
  (CallFunction|SetTeleportParaSvr StartPos EndPos MeshOffset))

(event EventPlaceTargetPos
  (params (TargetLoc :type Vector) (TargetRot :type Rotator :default "0, 0, 0") (ValidateTarget :type Boolean))
  ;[1 1 1] 设置指示位置
  (CallFunction|ShowRingMuilticast TargetLoc ValidateTarget))

(event EventActiveSkill
  (|CallParentFunction)
  (Development|SetHiddeninGame (Variables|Default|GetDefaultSceneRoot) false true))

(event EventDeactiveSkill
  (|CallParentFunction)
  (Development|SetHiddeninGame (Variables|Default|GetDefaultSceneRoot) true true))

(fn ConstructionScript
  (Development|SetHiddeninGame (Variables|Default|GetDefaultSceneRoot) true true)
  (bind _returnvalue (Rendering|Material|CreateDynamicMaterialInstance (Variables|Default|GetTeleportTargetCircle) 0 0 :!class /Script/Engine.PrimitiveComponent))
  (Variables|Default|SetDMI_TargetCurcle _returnvalue))