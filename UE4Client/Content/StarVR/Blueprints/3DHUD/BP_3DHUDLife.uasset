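; A 3D HUD health display that shows a life percentage as text, an arc bar, a blood panel and sliding arrows.
; The construction script creates dynamic materials and caches arrow transforms; SetHpDisplay clamps the value and updates text and visuals.
; SetHpBarScale drives arc fill and threshold color, lerps side arrows toward the center, and selects blood atlas cells via a Translation parameter.
; Box overlaps set a trend, but its fill/drain logic is unconnected.
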(event OnComponentBeginOverlap(Box)
  (params (OtherActor :type Actor%20Object%20Reference) (OtherComp :type Primitive%20Component%20Object%20Reference) (OtherBodyIndex :type Integer) (bFromSweep :type Boolean) (SweepResult :type Hit%20Result%20Structure%20%28by%20ref%29))
  (if (Variables|Test|GetIsCome)
    (Variables|Numric|SetNumTrend "NewEnumerator1")
    (Variables|Test|SetIsCome false)
    (else
      (Variables|Numric|SetNumTrend "NewEnumerator2")
      (Variables|Test|SetIsCome true))))

(event OnComponentEndOverlap(Box)
  (params (OtherActor :type Actor%20Object%20Reference) (OtherComp :type Primitive%20Component%20Object%20Reference) (OtherBodyIndex :type Integer))
  (Variables|Numric|SetNumTrend "NewEnumerator0"))

(event Custom|Construnct
  (bind _returnvalue (Rendering|Material|CreateDynamicMaterialInstance (Variables|Default|GetHPPanel) 0 "/Game/StarVR/Materials/3DHUD/M_DynamicBlood.M_DynamicBlood" :!class /Script/Engine.PrimitiveComponent))
  (bind _output_get (Variables|HPPanel|SetDynamicBloodMat _returnvalue))
  (Rendering|Material|SetVectorParameterValue _output_get "Translation" (Math|Color|MakeColor (Math|Conversions|ToFloat(Integer) (Variables|HPPanel|Getrow)) (Math|Conversions|ToFloat(Integer) (Variables|HPPanel|Getcol)) 0.0) :!class /Script/Engine.MaterialInstanceDynamic)
  (Rendering|Material|SetMaterial (Variables|Default|GetHPPanel) 0 (Variables|HPPanel|GetDynamicBloodMat))
  (bind _returnvalue_2 (Rendering|Material|CreateDynamicMaterialInstance (Variables|Default|GethpFore) 0 "/Game/StarVR/Materials/3DHUD/M_HPArc_Inst_Fore.M_HPArc_Inst_Fore" :!class /Script/Engine.PrimitiveComponent))
  (Variables|HPBar|SetHPBarFore _returnvalue_2)
  (bind _returnvalue_3 (Rendering|Material|GetScalarParameterValue (Variables|HPBar|GetHPBarFore) "DisplayAlpha" :!class /Script/Engine.MaterialInstanceDynamic))
  (Variables|Numric|SetHPFullFactor _returnvalue_3)
  (bind _returnvalue_4 (Rendering|Material|GetVectorParameterValue (Variables|HPBar|GetHPBarFore) "DisplayColor" :!class /Script/Engine.MaterialInstanceDynamic))
  (Variables|HPBar|SetHPBarColor _returnvalue_4)
  (Variables|HPBar|SetLeftArrowTrans (Transformation|GetRelativeTransform (Variables|Default|GetSM_LeftArrow)))
  (Variables|HPBar|SetRightArrowTrans (Transformation|GetRelativeTransform (Variables|Default|GetSM_RightArrow)))
  (Variables|HPBar|SetArrowDestTrans (Transformation|GetRelativeTransform (Variables|Default|GetSM_CenterArrow))))

(event Custom|SetHpDisplay
  (params (NewParam :type Float%20%28single-precision%29))
  (bind _output_get (Variables|Numric|SetIncomeNum (Math|Float|Clamp(Float) NewParam 0.0 1e+02)))
  (CallFunction|SetHpBarScale (+ (Variables|Numric|GetHealthPoint) (Math|Float|Truncate _output_get)))
  (Rendering|Components|TextRender|SetText (Variables|Default|GetTextRender) (Utilities|Text|ToText(String) (Utilities|String|Append (Utilities|String|ToString(Integer) (+ (Variables|Numric|GetHealthPoint) (Math|Float|Truncate _output_get))) "%"))))

(event Custom|SetHpBarScale
  (params (DisplayHPNum :type Integer))
  (bind _returnvalue (/ 0.5 13.0))
  (bind _hpbarfore (Variables|HPBar|GetHPBarFore))
  (bind _hpfullfactor (Variables|Numric|GetHPFullFactor))
  (bind _incomenum (Variables|Numric|GetIncomeNum))
  (bind _dynamicbloodmat (Variables|HPPanel|GetDynamicBloodMat))
  (bind _dynamicbloodmat_2 (Variables|HPPanel|GetDynamicBloodMat))
  (bind _returnvalue_2 (* _hpfullfactor _incomenum))
  (bind _returnvalue_3 (/ _returnvalue_2 1e+02))
  (bind _returnvalue_4 (/ _returnvalue_3 _returnvalue))
  (bind _returnvalue_5 (* _returnvalue_3 2.0))
  (bind _returnvalue_6 (Math|Float|Truncate _returnvalue_4))
  (bind _returnvalue_7 (- 12 _returnvalue_6))
  (Rendering|Material|SetScalarParameterValue _hpbarfore "DisplayAlpha" _returnvalue_3 :!class /Script/Engine.MaterialInstanceDynamic)
  (if (and (<= _returnvalue_3 0.5) (> _returnvalue_3 0.3))
    (Rendering|Material|SetVectorParameterValue _hpbarfore "DisplayColor" "(R=0.000000,G=1.000000,B=0.000000,A=1.000000)" :!class /Script/Engine.MaterialInstanceDynamic)
    (elif (and (<= _returnvalue_3 0.3) (> _returnvalue_3 0.1))
      (Rendering|Material|SetVectorParameterValue _hpbarfore "DisplayColor" "(R=0.926359,G=1.000000,B=0.000000,A=1.000000)" :!class /Script/Engine.MaterialInstanceDynamic)
      (else
        (Rendering|Material|SetVectorParameterValue _hpbarfore "DisplayColor" "(R=1.000000,G=0.000000,B=0.000000,A=1.000000)" :!class /Script/Engine.MaterialInstanceDynamic))))
  (Transformation|SetRelativeTransform (Variables|Default|GetSM_LeftArrow) (Math|Transform|Lerp(Transform) (Variables|HPBar|GetArrowDestTrans) (Variables|HPBar|GetLeftArrowTrans) _returnvalue_5) false false)
  (Transformation|SetRelativeTransform (Variables|Default|GetSM_RightArrow) (Math|Transform|Lerp(Transform) (Variables|HPBar|GetArrowDestTrans) (Variables|HPBar|GetRightArrowTrans) _returnvalue_5) false false)
  (if (== DisplayHPNum 0)
    (Rendering|Material|SetVectorParameterValue _dynamicbloodmat_2 "Translation" (Math|Color|MakeColor 1.0 3.0 0.0) :!class /Script/Engine.MaterialInstanceDynamic)
    (Rendering|Material|SetMaterial (Variables|Default|GetHPPanel) 0 _dynamicbloodmat_2)
    (else
      (Rendering|Material|SetVectorParameterValue _dynamicbloodmat "Translation" (Math|Color|MakeColor (Math|Conversions|ToFloat(Integer) (Math|Integer|%(Integer) _returnvalue_7 4)) (Math|Conversions|ToFloat(Integer) (/ _returnvalue_7 4)) 0.0) :!class /Script/Engine.MaterialInstanceDynamic)
      (Rendering|Material|SetMaterial (Variables|Default|GetHPPanel) 0 _dynamicbloodmat))))

(event EventBeginPlay)

(event EventTick
  (params (DeltaSeconds :type Float%20%28single-precision%29)))

(fn ConstructionScript
  (Rendering|Components|TextRender|SetText (Variables|Default|GetTextRender) (Variables|Numric|GetInitWording))
  (CallFunction|Construnct))