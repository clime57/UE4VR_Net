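; BP_WeaponImpact is a weapon impact effects Blueprint that reacts to a hit based on the surface struck.
; ImpactHit uses the physical material's surface type to select a particle effect and spawns it at the impact point along the normal.
; Selectors only assign assets for the Default surface.
; The randomly rolled, attached decal logic is disconnected, the sound selector is never called, and blood assets are unused.
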(event Custom|ImpactHit
  (params (HitResult :type Hit%20Result%20Structure))
  (bind (_bblockinghit _binitialoverlap _time _location _impactpoint _normal _impactnormal _physmat _hitactor _hitcomponent _hitbonename) (Collision|BreakHitResult HitResult))
  (bind _surfacetype (Variables|/Script/Engine.PhysicalMaterial|GetSurfaceType _physmat))
  (bind _particle (CallFunction|GetImpactFX _surfacetype))
  (Utilities|IsValid _physmat
    (:Is%20Valid
      (Utilities|FlowControl|Sequence
        (:then_0
          (Utilities|IsValid _particle
            (:Is%20Valid
              (Effects|SpawnEmitteratLocation _particle _impactpoint (Math|Rotator|MakeRotfromZ _impactnormal)))))))))

(fn ConstructionScript)

(fn GetImpactFX
  (params (SurfaceType :type EPhysicalSurface%20Enum))
  (return (Utilities|Select :Index SurfaceType :SurfaceType_Default (Variables|Default|GetDefaultFX) :SurfaceType1 0 :SurfaceType2 0)))

(fn GetImpactSound
  (params (SurfaceType :type EPhysicalSurface%20Enum))
  (return (Utilities|Select :Index SurfaceType :SurfaceType_Default (Variables|Default|GetDefaultSound) :SurfaceType1 0 :SurfaceType2 0)))

(fn GetImpactDecal
  (params (Type :type EPhysicalSurface%20Enum))
  (return (Utilities|Select :Index Type :SurfaceType_Default (Variables|Default|GetDefaultDecal) :SurfaceType1 "" :SurfaceType2 "")))