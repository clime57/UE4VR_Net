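; Game instance that manages multiplayer sessions, with helpers for a world-space scoreboard and cursor clicks.
; It hosts listen-server levels, joins the first or a chosen session, reports searches through FindSessionSuccess even on failure, and returns to the main menu.
; Network and travel errors print and destroy the session.
; The scoreboard actor spawns once and repositions ahead of the player's head using yaw only, while clicks reach hit actors through BPI_UI.
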(event Custom|CreateSession
  (params (Level :type Name))
  (|Session (Game|GetPlayerController 0) 4 (Variables|Default|GetUseLan)
    (:OnSuccess
      (Game|OpenLevel(byName) Level true "listen"))
    (:OnFailure
      (Development|PrintString "Create session failed!!!" true true "(R=0.000000,G=0.660000,B=1.000000,A=1.000000)" 1e+01))))

(event Custom|JoinSession
  (params (SessionResult :type Blueprint%20Session%20Result%20Structure))
  (|JoinSession (Game|GetPlayerController 0) SessionResult))

(event Custom|FindAndJoinSession
  (bind _results (|FindSessions (Game|GetPlayerController 0) 1 (Variables|Default|GetUseLan))
    (:OnSuccess
      (if (>= (Utilities|Array|Length _results) 1)
        (|JoinSession (Game|GetPlayerController 0) (Utilities|Array|Get(acopy) _results))
        (else
          (Development|PrintString "Find Sessions None" true true "(R=0.000000,G=0.660000,B=1.000000,A=1.000000)" 1e+01))))))

(event Custom|FindSessions
  (bind _results (|FindSessions (Game|GetPlayerController 0) 20 (Variables|Default|GetUseLan))
    (:OnSuccess
      (bind _output_get (Variables|Default|SetSessionResults _results))
      (Default|CallFindSessionSuccess _output_get))
    (:OnFailure
      (Default|CallFindSessionSuccess _results))))

(event Custom|ReturnToMainMenu
  (|DestroySession (Game|GetPlayerController 0)
    (:OnSuccess
      (Game|OpenLevel(byName) "L_MainMenu"))
    (:OnFailure
      (Development|PrintString "End session failed!!!" true true "(R=0.000000,G=0.660000,B=1.000000,A=1.000000)" 1e+01))))

(event Custom|ShowScoreBoard
  (params (Show :type Boolean))
  (bind _transform (Class|BPIPlayerPawn|GetHeadTransform(Message) (Game|Player|GetPlayerPawn 0)))
  (Utilities|IsValid (Variables|Default|GetScoreBoard)
    (:Is%20Valid
      _)
    (:Is%20Not%20Valid
      (bind _returnvalue (Game|SpawnActorfromClass "/Game/BlackShield/Blueprints/UI/ScoreBoard/BP_BoardUI.BP_BoardUI_C" (Math|Transform|MakeTransform (+ (.Location (Math|Transform|BreakTransform _transform)) (* (Math|Vector|GetForwardVector (Math|Rotator|MakeRotator 0.0 0.0 (.Yaw (Math|Rotator|BreakRotator (.Rotation (Math|Transform|BreakTransform _transform)))))) 3e+02)) (Math|Rotator|MakeRotator 0.0 0.0 (.Yaw (Math|Rotator|BreakRotator (.Rotation (Math|Transform|BreakTransform _transform)))))) "AlwaysSpawn" 0 0))
      (Variables|Default|SetScoreBoard _returnvalue)))
  (Transformation|SetActorTransform (Variables|Default|GetScoreBoard) (Math|Transform|MakeTransform (+ (.Location (Math|Transform|BreakTransform _transform)) (* (Math|Vector|GetForwardVector (Math|Rotator|MakeRotator 0.0 0.0 (.Yaw (Math|Rotator|BreakRotator (.Rotation (Math|Transform|BreakTransform _transform)))))) 3e+02)) (Math|Rotator|MakeRotator 0.0 0.0 (.Yaw (Math|Rotator|BreakRotator (.Rotation (Math|Transform|BreakTransform _transform)))))))
  (Default|ShowBoard (Variables|Default|GetScoreBoard) Show))

(event Custom|ButtonDown
  (bind _returnvalue (Game|GetPlayerController 0))
  (bind (_hitresult _returnvalue_2) (Game|Player|GetHitResultUnderCursorbyChannel _returnvalue "TraceTypeQuery1" true))
  (bind _hitactor (Collision|BreakHitResult _hitresult))
  (if _returnvalue_2
    (if (Utilities|DoesObjectImplementInterface _hitactor "/Game/BlackShield/Blueprints/UI/BPI_UI.BPI_UI_C")
      (Class|BPIUI|OnClickButton(Message) _hitactor))))

(event EventHandleTravelError
  (params (FailureType :type ETravelFailure%20Enum :default "NoLevel"))
  (Development|PrintString (Utilities|String|Append "TravelError" (Utilities|String|EnumtoString FailureType)) true true "(R=0.000000,G=0.660000,B=1.000000,A=1.000000)" 1e+01)
  (|DestroySession (Game|GetPlayerController 0)))

(event EventHandleNetworkError
  (params (FailureType :type ENetworkFailure%20Enum :default "NetDriverAlreadyExists") (bIsServer :type Boolean))
  (Development|PrintString (Utilities|String|Append "NetworkError" (Utilities|String|EnumtoString FailureType)) true true "(R=0.000000,G=0.660000,B=1.000000,A=1.000000)" 1e+01)
  (|DestroySession (Game|GetPlayerController 0)))