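; BP_PlayerStateNet is the networked player state that tracks a player's score, kills, assists, deaths and readiness to play.
; Simple events and functions increment kills, deaths and score, while a test-only function randomizes the kill, assist and death counts.
; GetBoardData packs the player index and those three counts into a semicolon-separated string for a board.
; A RepNotify on IsReadyForPlay passes readiness changes to BP_NetGameInstance.
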(event Custom|AddKillNum
  (Variables|Default|SetPlayerKillNum (+ (Variables|Default|GetPlayerKillNum) 1)))

(event Custom|AddDeadNum
  (Variables|Default|SetPlayerDeadNum (+ (Variables|Default|GetPlayerDeadNum) 1)))

(fn ConstructionScript)

(fn IncrementScore
  (Variables|Default|SetPlayerScore (+ (Variables|Default|GetPlayerScore) 1)))

(fn GetBoardData
  (return (Class|VictoryBPFunctionLibrary|AppendMultiple (Utilities|String|ToString(Integer) (Variables|Default|GetPlayerIndex)) ";" (Utilities|String|ToString(Integer) (Variables|Default|GetPlayerKillNum)) ";" (Utilities|String|ToString(Integer) (Variables|Default|GetPlayerAssistNum)) ";" (Utilities|String|ToString(Integer) (Variables|Default|GetPlayerDeadNum)))))

(fn RandomBoardData
  (bind _returnvalue (Math|Random|RandomIntegerinRange 0 20))
  ;[1 1 1] 仅用于测试
  (Variables|Default|SetPlayerKillNum _returnvalue)
  (Variables|Default|SetPlayerAssistNum _returnvalue)
  (Variables|Default|SetPlayerDeadNum _returnvalue))

(fn OnRepIsReadyforPlay
  (bind _asbp_net_game_instance (Utilities|Casting|CastToBP_NetGameInstance (Game|GetGameInstance)))
  (Default|CallReadyPlayingChange _asbp_net_game_instance self))