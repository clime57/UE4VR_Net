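; VR motion recorder that stores timestamped head and both-hand locations and rotations and reads them back sample by sample.
; Add appends samples to parallel arrays up to a maximum count, while GetCurent, PopFromHead and MoveNext read through them with a shared cursor.
; Save writes delimited lines to Recored.txt in the game root, rewriting the file on every loop pass.
; Load parses that file back into the pose arrays, discarding timestamps.
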(event EventBeginPlay)

(event EventTick
  (params (DeltaSeconds :type Float%20%28single-precision%29)))

(fn Save
  (for _index (range 0 (- (Utilities|Array|Length (Variables|Default|GetHead_Loc)) 1))
    (Utilities|Array|Add (LocalVariables|GetSaveTextArray) (Utilities|String|Append (Utilities|String|ToString(Float) (Utilities|Array|Get(acopy) (Variables|Default|GetTime) _index)) "|" (Utilities|String|ToString(Vector) (Utilities|Array|Get(acopy) (Variables|Default|GetHead_Loc) _index)) ";" (Utilities|String|ToString(Rotator) (Utilities|Array|Get(acopy) (Variables|Default|GetHead_Rot) _index)) ";" (Utilities|String|ToString(Vector) (Utilities|Array|Get(acopy) (Variables|Default|GetHand_Loc_L) _index)) ";" (Utilities|String|ToString(Rotator) (Utilities|Array|Get(acopy) (Variables|Default|GetHand_Rot_L) _index)) ";" (Utilities|String|ToString(Vector) (Utilities|Array|Get(acopy) (Variables|Default|GetHand_Loc_R) _index)) ";" (Utilities|String|ToString(Rotator) (Utilities|Array|Get(acopy) (Variables|Default|GetHand_Rot_R) _index))))
    (Class|VictoryBPFunctionLibrary|FileIOSaveStringArraytoFile (Class|VictoryBPFunctionLibrary|VictoryPathsGameRootDirectory) "Recored.txt" (LocalVariables|GetSaveTextArray) true)))

(fn Load
  (for _array_element (.StringArray (Class|VictoryBPFunctionLibrary|LoadStringArrayfromFile (Utilities|String|Append (Class|VictoryBPFunctionLibrary|VictoryPathsGameRootDirectory) "/Recored.txt") true))
    (bind _output_get (LocalVariables|SetcurStr (Class|VictoryBPFunctionLibrary|StringExplodeString (Utilities|Array|Get(acopy) (Class|VictoryBPFunctionLibrary|StringExplodeString _array_element "|" 0 false) 1) ";" 0 false)))
    (Utilities|Array|Add (Variables|Default|GetHead_Loc) (.ConvertedVector (Class|VictoryBPFunctionLibrary|ConversionsStringtoVector (Utilities|Array|Get(acopy) _output_get))))
    (Utilities|Array|Add (Variables|Default|GetHead_Rot) (.ConvertedRotator (Class|VictoryBPFunctionLibrary|ConversionsStringtoRotator (Utilities|Array|Get(acopy) _output_get 1))))
    (Utilities|Array|Add (Variables|Default|GetHand_Loc_L) (.ConvertedVector (Class|VictoryBPFunctionLibrary|ConversionsStringtoVector (Utilities|Array|Get(acopy) _output_get 2))))
    (Utilities|Array|Add (Variables|Default|GetHand_Rot_L) (.ConvertedRotator (Class|VictoryBPFunctionLibrary|ConversionsStringtoRotator (Utilities|Array|Get(acopy) _output_get 3))))
    (Utilities|Array|Add (Variables|Default|GetHand_Loc_R) (.ConvertedVector (Class|VictoryBPFunctionLibrary|ConversionsStringtoVector (Utilities|Array|Get(acopy) _output_get 4))))
    (Utilities|Array|Add (Variables|Default|GetHand_Rot_R) (.ConvertedRotator (Class|VictoryBPFunctionLibrary|ConversionsStringtoRotator (Utilities|Array|Get(acopy) _output_get 5))))))

(fn PopfromHead
  (bind (_head_loc _head_rot _hand_loc_l _hand_rot_l _hand_loc_r _hand_rot_r) (CallFunction|GetCurent))
  (Variables|Default|SetCurPos (+ (Variables|Default|GetCurPos) 1))
  (return _head_loc _head_rot _hand_loc_l _hand_rot_l _hand_loc_r _hand_rot_r))

(fn GetCurent
  (bind _curpos (Variables|Default|GetCurPos))
  (bind _positions (LocalVariables|GetPositions))
  (bind _rotators (LocalVariables|GetRotators))
  (Utilities|Array|Add (LocalVariables|GetPositions) (Utilities|Array|Get(acopy) (Variables|Default|GetHead_Loc) _curpos))
  (Utilities|Array|Add (LocalVariables|GetRotators) (Utilities|Array|Get(acopy) (Variables|Default|GetHead_Rot) _curpos))
  (Utilities|Array|Add (LocalVariables|GetPositions) (Utilities|Array|Get(acopy) (Variables|Default|GetHand_Loc_L) _curpos))
  (Utilities|Array|Add (LocalVariables|GetRotators) (Utilities|Array|Get(acopy) (Variables|Default|GetHand_Rot_L) _curpos))
  (Utilities|Array|Add (LocalVariables|GetPositions) (Utilities|Array|Get(acopy) (Variables|Default|GetHand_Loc_R) _curpos))
  (Utilities|Array|Add (LocalVariables|GetRotators) (Utilities|Array|Get(acopy) (Variables|Default|GetHand_Rot_R) _curpos))
  (return (Utilities|Array|Get(acopy) _positions) (Utilities|Array|Get(acopy) _rotators) (Utilities|Array|Get(acopy) _positions 1) (Utilities|Array|Get(acopy) _rotators 1) (Utilities|Array|Get(acopy) _positions 2) (Utilities|Array|Get(acopy) _rotators 2)))

(fn Add
  (params (Head_Loc :type Vector) (Head_Rot :type Rotator) (Hand_Loc_L :type Vector) (Hand_Rot_L :type Rotator) (Hand_loc_R :type Vector) (Hand_Rot_R :type Rotator))
  (if (< (Variables|Default|GetCurPos) (Variables|Default|GetRecoredMaxCount))
    (Utilities|Array|Add (Variables|Default|GetHead_Loc) Head_Loc)
    (Utilities|Array|Add (Variables|Default|GetHead_Rot) Head_Rot)
    (Utilities|Array|Add (Variables|Default|GetHand_Loc_L) Hand_Loc_L)
    (Utilities|Array|Add (Variables|Default|GetHand_Rot_L) Hand_Rot_L)
    (Utilities|Array|Add (Variables|Default|GetHand_Loc_R) Hand_loc_R)
    (Utilities|Array|Add (Variables|Default|GetHand_Rot_R) Hand_Rot_R)
    (Utilities|Array|Add (Variables|Default|GetTime) (Utilities|Time|GetGameTimeinSeconds))
    (bind _output_get (Variables|Default|SetCurPos (+ (Variables|Default|GetCurPos) 1)))
    (Development|PrintString (Utilities|String|ToString(Integer) _output_get))))

(fn MoveNext
  (if (< (Variables|Default|GetCurPos) (Utilities|Array|Length (Variables|Default|GetHead_Loc)))
    (Variables|Default|SetCurPos (+ (Variables|Default|GetCurPos) 1))
    (LocalVariables|Set_isEnd false)
    (else
      (LocalVariables|Set_isEnd true)))
  (return (LocalVariables|Get_isEnd)))