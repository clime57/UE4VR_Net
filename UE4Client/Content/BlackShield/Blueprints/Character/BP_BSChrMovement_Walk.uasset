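; BP_BSChrMovement_Walk is a BlackShield character Blueprint, named as the walking movement variant, that layers an overhead health bar onto its parent class.
; Each Tick runs the parent logic, then casts the child actor to BP_OHHPBar and updates it with the current-to-initial health ratio.
; An unconnected "Create Foot Fire" chain would attach particle systems to both toe sockets but never runs.
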(event EventBeginPlay
  (|CallParentFunction))

(event EventTick
  (params (DeltaSeconds :type Float%20%28single-precision%29))
  (|CallParentFunction DeltaSeconds)
  (bind _asbp_ohhpbar (Utilities|Casting|CastToBP_OHHPBar (Variables|/Script/Engine.ChildActorComponent|GetChildActor (Variables|Default|GetChildActor))))
  (Default|Update _asbp_ohhpbar (/ (Math|Conversions|ToFloat(Integer) (Variables|Default|GetCurentHealth)) (Math|Conversions|ToFloat(Integer) (Variables|Default|GetInitHealth)))))

(fn ConstructionScript
  (|CallParentFunction))