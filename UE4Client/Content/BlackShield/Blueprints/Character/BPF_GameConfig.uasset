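; Blueprint function library for BlackShield that resolves the configured input mode and provides small shared helpers.
; GetInputType reads the mode from a custom config through the Victory plugin, defaulting to HTC Vive over Record or Keyboard.
; GetCameraPose uses that mode to return either the tracked headset pose offset by camera manager location, or the camera manager's view.
; Other helpers check actor tags and convert level names to display text.
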(fn GetInputType
  (bind (_isvalid _returnvalue) (Class|VictoryBPFunctionLibrary|VictoryGetCustomConfigVarInt "Input" "InputType"))
  (if _isvalid
    (LocalVariables|SetConfigValue _returnvalue)
    (if (== (LocalVariables|GetConfigValue) 0)
      (return "NewEnumerator0")
      (elif (== (LocalVariables|GetConfigValue) 1)
        (return "NewEnumerator1")
        (elif (== (LocalVariables|GetConfigValue) 2)
          (return "NewEnumerator2")
          (else
            (return "NewEnumerator0")))))
    (else
      (return "NewEnumerator0"))))

(fn ActorHasTag
  (params (Actor :type Actor%20Object%20Reference) (Tag :type Name))
  (Utilities|IsValid Actor
    (:Is%20Valid
      (if (or (Utilities|Name|Equal(Name) Tag "None") (Utilities|Name|Equal(Name) Tag ""))
        (return false)
        (else
          (bind _array_element (Utilities|Array|ForEachLoopwithBreak (Variables|/Script/Engine.Actor|GetTags Actor) :!label _label)
            (:LoopBody
              (if (Utilities|Name|Equal(Name) _array_element Tag)
                (LocalVariables|SetHasTag true)
                (goto _label Break)))
            (:Completed
              (return (LocalVariables|GetHasTag)))))))
    (:Is%20Not%20Valid
      (return false))))

(fn GetCameraPose
  (bind (_outposition _outorientation) (Class|SteamVRFunctionLibrary|GetTrackedDevicePositionandOrientation))
  (bind _returnvalue (Game|GetPlayerCameraManager 0))
  (bind _returnvalue_2 (Camera|GetCameraLocation _returnvalue))
  (bind _returnvalue_3 (Camera|GetCameraRotation _returnvalue))
  (switch Utilities|FlowControl|Switch|SwitchonInputTypeEnum (CallFunction|GetInputType)
    (:NewEnumerator0
      (return (+ _outposition (Transformation|GetActorLocation _returnvalue)) _outorientation))
    (:NewEnumerator1
      (return _returnvalue_2 _returnvalue_3))
    (:NewEnumerator2
      (return _returnvalue_2 _returnvalue_3))))

(fn GetLevelShowName
  (params (LevelString :type Name))
  (return (Utilities|Text|ToText(Name) LevelString)))