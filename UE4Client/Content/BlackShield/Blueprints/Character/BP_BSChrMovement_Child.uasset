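; Child Blueprint of the BlackShield character movement actor that adds its material and particle-style effects for death, teleport and body translucency.
; The construction script turns every mesh material into a dynamic instance, whose Power parameter DeathEffect animates through a timeline.
; TeleportEffect activates PMove for one second, and the translucency override swaps all but three material slots on the locally controlled character.
; Leftover directional movement and animation-feeding logic is disconnected.
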(event Custom|SetBodyTransluncyClient
  ;[1 1 1] Override
  (CallFunction|SetBodyTransluncy))

(event EventDeathEffect
  (bind _newtrack_1 (Timeline|Timeline_0 Play)
    (:Update
      (for _array_element (Variables|Default|GetDymicMaterials)
        (Rendering|Material|SetScalarParameterValue _array_element "Power" (* _newtrack_1 1e+01) :!class /Script/Engine.MaterialInstanceDynamic)))))

(event EventBeginPlay
  (Utilities|FlowControl|Sequence
    (:then_0
      (|CallParentFunction))))

(event EventActorBeginOverlap
  (params (OtherActor :type Actor%20Object%20Reference)))

(event EventTeleportEffect
  (bind _p_move (Variables|Default|GetP_Move))
  (Components|Activation|SetActive _p_move true true)
  (Utilities|FlowControl|Delay 1.0)
  (Components|Activation|SetActive _p_move false true))

(fn ConstructionScript
  (Variables|Default|SetMeshType "NewEnumerator0")
  (Variables|Default|SetMeshAngle 0.0)
  (|CallParentFunction)
  (for (_array_element _array_index) (Rendering|Material|GetMaterials (Variables|Default|GetSkeletalMesh))
    (bind _returnvalue (Rendering|Material|CreateDynamicMaterialInstance (Variables|Default|GetSkeletalMesh) _array_index _array_element :!class /Script/Engine.PrimitiveComponent))
    (Rendering|Material|SetScalarParameterValue _returnvalue "Power" (* (Variables|Default|GetDefaltPower) 1e+01) :!class /Script/Engine.MaterialInstanceDynamic)
    (Utilities|Array|Add (Variables|Default|GetDymicMaterials) _returnvalue)))

(fn SetBodyTransluncy
  (if (Pawn|IsLocallyControlled)
    (for (_ _array_index) (Rendering|Material|GetMaterials (Variables|Default|GetSkeletalMesh))
      (if (not (Math|Boolean|ORBoolean (== _array_index 5) (== _array_index 6) (== _array_index 9)))
        (Rendering|Material|SetMaterial (Variables|Default|GetSkeletalMesh) _array_index "/Game/BlackShield/Materials/M_NewMaterial.M_NewMaterial")))))