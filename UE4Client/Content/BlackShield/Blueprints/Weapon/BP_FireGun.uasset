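; BP_FireGun is a flamethrower-style weapon that deals continuous damage along its forward direction while active.
; Activating or deactivating it sets IsFire and toggles the particle system through ActiveFireClient.
; On authority, a looping cooldown timer runs a forward multi sphere trace while firing, ignoring the owning character and sending HitReactionMessage to each hit with DPS scaled by the cooldown.
; The trace's debug draw is left on, and the IsFire OnRep is empty.
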(event Custom|OpenFire
  (bind _output_get (Variables|Default|SetisFire true))
  (CallFunction|ActiveFireClient _output_get))

(event Custom|ActiveFireClient
  (params (bNewActive :type Boolean))
  (Components|Activation|SetActive (Variables|Default|GetParticleSystem) bNewActive true))

(event Custom|FireInClient
  (bind _returnvalue (Transformation|GetActorLocation))
  (Networking|SwitchHasAuthority
    (:Authority
      (if (Variables|Default|GetisFire)
        (bind _outhits (Class|KismetSystemLibrary|SphereTraceMultiNEW _returnvalue (+ _returnvalue (Math|Vector|RotateVector "800.000000,0.000000, 0" (Transformation|GetActorRotation))) 3e+01 "TraceTypeQuery4" false (Utilities|Array|MakeArray (Variables|Default|GetCharacterActor)) "ForOneFrame" true))
        (for _array_element _outhits
          (Class|BPIImpact|HitReaction(Message) (.HitActor (Collision|BreakHitResult _array_element)) "None" (.ImpactPoint (Collision|BreakHitResult _array_element)) "0, 0, 0" (* (Variables|Default|GetDPS) (Variables|Default|GetCoolDown)) (Variables|Default|GetCharacterActor)))))))

(event Custom|CeaseFire
  (bind _output_get (Variables|Default|SetisFire false))
  (CallFunction|ActiveFireClient _output_get))

(event EventBeginPlay
  (Networking|SwitchHasAuthority
    (:Authority
      (Utilities|Time|SetTimerbyEvent (delegate Custom|FireInClient) (Variables|Default|GetCoolDown) true))))

(event EventActiveWeapon
  (CallFunction|OpenFire))

(event EventDeactiveWeapon
  (CallFunction|CeaseFire))

(fn ConstructionScript)

(fn OnRepIsFire)