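; BP_WeaponGun is an automatic gun that fires bullets and muzzle effects while the weapon is active.
; A looping timer at the Speed interval checks the BulletActive flag, which activation and deactivation toggle.
; Each shot decrements the magazine, spawns BP_GunBullet on authority only, and plays a scaled-down emitter.
; ReloadPower refills the magazine and GetState reports it, but the empty-magazine check is disconnected, so ammo never limits firing.
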(event Custom|SpawnBullet
  (bind _gun (Variables|Default|GetGun))
  (bind _returnvalue (Transformation|GetWorldTransform _gun))
  (bind (_location _rotation) (Math|Transform|BreakTransform _returnvalue))
  (if (Variables|Default|GetBulletActive)
    (Math|Integer|DecrementInt (Variables|Default|GetCurBulletNumMagazine)
      (:%20%20
        (Networking|SwitchHasAuthority
          (:Authority
            (Game|SpawnActorfromClass "/Game/BlackShield/Blueprints/Weapon/BP_GunBullet.BP_GunBullet_C" (Math|Transform|MakeTransform _location _rotation "1.000000,1.000000,1.000000") "Undefined" 0 (Variables|Default|GetCharacterActor) 0))
          (:Remote
            _))
        (CallFunction|SpawnEmitter)))))

(event Custom|SpawnEmitter
  (bind _gun (Variables|Default|GetGun))
  (bind _returnvalue (Transformation|GetWorldTransform _gun))
  (bind (_location _rotation) (Math|Transform|BreakTransform _returnvalue))
  (bind _returnvalue_2 (Effects|SpawnEmitteratLocation (Variables|Default|GetFiringEffect) _location _rotation))
  (Transformation|SetWorldScale3D _returnvalue_2 "0.500000,0.500000,0.500000"))

(event Custom|CeaseFire
  (Variables|Default|SetBulletActive false))

(event Custom|OpenFire
  (Variables|Default|SetBulletActive true))

(event EventBeginPlay
  (Utilities|Time|SetTimerbyEvent (delegate Custom|SpawnBullet) (Variables|Default|GetSpeed) true))

(event EventActiveWeapon
  (CallFunction|OpenFire))

(event EventDeactiveWeapon
  (CallFunction|CeaseFire))

(event EventReloadPower
  (Variables|Default|SetCurBulletNumMagazine (Variables|Default|GetMaxBulletNumMagazine)))

(fn ConstructionScript
  (Variables|Default|SetCurBulletNumMagazine (Variables|Default|GetMaxBulletNumMagazine)))

(fn GetState
  (return (Variables|Default|GetMaxBulletNumMagazine) (Variables|Default|GetCurBulletNumMagazine)))