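; BP_WeaponManager manages a character's current weapon and skill actors and forwards activate, deactivate, cast, place and reload calls to them.
; Changing the weapon or skill index triggers an OnRep that destroys the old actor, spawns the selected class and assigns the Character.
; Actions relay through Multicast events, while pose and target updates skip the locally controlled client, which has separate Local events.
; Destroying the manager also destroys both spawned actors.
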(event Custom|DeactiveCurrentWeapon_Multicast
  (bind _currentweaponactor (Variables|Default|GetCurrentWeaponActor))
  (Utilities|IsValid _currentweaponactor
    (:Is%20Valid
      (Default|DeactiveWeapon _currentweaponactor))))

(event Custom|PlaceTargetPos_Multicast
  (params (TargetPos :type Vector) (TargetRot :type Rotator) (ValidatePos :type Boolean))
  (bind _currentskillactor (Variables|Default|GetCurrentSkillActor))
  (if (not (CallFunction|IsLocally))
    (Utilities|IsValid _currentskillactor
      (:Is%20Valid
        (Default|PlaceTargetPos _currentskillactor TargetPos TargetRot ValidatePos)))))

(event Custom|PlaceTargetPos_Local
  (params (TargetPos :type Vector) (TargetRot :type Rotator) (ValidatePos :type Boolean))
  (bind _currentskillactor (Variables|Default|GetCurrentSkillActor))
  (Utilities|IsValid _currentskillactor
    (:Is%20Valid
      (Default|PlaceTargetPos _currentskillactor TargetPos TargetRot ValidatePos))))

(event Custom|ChangeSkill
  (params (SkillIndex :type SkillType%20Enum))
  (Variables|Default|SetSkillIndex SkillIndex))

(event Custom|ActiveCurrentSkill
  (CallFunction|ActiveCurrentSkillMulticast))

(event Custom|DeactiveCurrentSkill
  (CallFunction|DeactiveCurrentSkillMulticast))

(event Custom|CastCurrentSkill
  (params (StartPos :type Vector) (EndPos :type Vector) (MeshOffset :type Vector))
  (bind _currentskillactor (Variables|Default|GetCurrentSkillActor))
  (Utilities|IsValid _currentskillactor
    (:Is%20Valid
      (Default|CastSkill _currentskillactor StartPos EndPos MeshOffset))))

(event Custom|PlaceTargetPos
  (params (TargetPos :type Vector) (TargetRot :type Rotator) (ValidatePos :type Boolean))
  (CallFunction|PlaceTargetPosMulticast TargetPos TargetRot ValidatePos))

(event Custom|ReloadCurentWeapon_Multicast
  (bind _currentweaponactor (Variables|Default|GetCurrentWeaponActor))
  (Utilities|IsValid _currentweaponactor
    (:Is%20Valid
      (Default|ReloadPower _currentweaponactor))))

(event Custom|UpdateCurentWeaponPose
  (params (Loc :type Vector) (Rot :type Rotator))
  (CallFunction|UpdateCurentWeaponPoseMulticast Loc Rot))

(event Custom|ActiveCurrentWeapon
  (CallFunction|ActiveCurrentWeaponMulticast))

(event Custom|DeactiveCurrentWeapon
  (CallFunction|DeactiveCurrentWeaponMulticast))

(event Custom|ReloadCurentWeapon
  (CallFunction|ReloadCurentWeaponMulticast))

(event Custom|UpdateCurentWeaponPose_Multicast
  (params (Loc :type Vector) (Rot :type Rotator))
  (bind _currentweaponactor (Variables|Default|GetCurrentWeaponActor))
  (if (not (CallFunction|IsLocally))
    (Utilities|IsValid _currentweaponactor
      (:Is%20Valid
        (Default|PlaceWeaponPos _currentweaponactor Loc Rot)))))

(event Custom|DeactiveCurrentSkill_Multicast
  (bind _currentskillactor (Variables|Default|GetCurrentSkillActor))
  (Utilities|IsValid _currentskillactor
    (:Is%20Valid
      (Default|DeactiveSkill _currentskillactor))))

(event Custom|UpdateCurentWeaponPose_Local
  (params (Loc :type Vector) (Rot :type Rotator))
  (bind _currentweaponactor (Variables|Default|GetCurrentWeaponActor))
  (Utilities|IsValid _currentweaponactor
    (:Is%20Valid
      (Default|PlaceWeaponPos _currentweaponactor Loc Rot))))

(event Custom|ActiveCurrentSkill_Multicast
  (bind _currentskillactor (Variables|Default|GetCurrentSkillActor))
  (Utilities|IsValid _currentskillactor
    (:Is%20Valid
      (Default|ActiveSkill _currentskillactor))))

(event Custom|ChangeWeapon
  (params (WeaponIndex :type WeaponType%20Enum))
  (Variables|Default|SetWeaponIndex WeaponIndex))

(event Custom|ActiveCurrentWeapon_Multicast
  (bind _currentweaponactor (Variables|Default|GetCurrentWeaponActor))
  (Utilities|IsValid _currentweaponactor
    (:Is%20Valid
      (Default|ActiveWeapon _currentweaponactor))))

(event EventDestroyed
  (bind _currentweaponactor (Variables|Default|GetCurrentWeaponActor))
  (bind _currentskillactor (Variables|Default|GetCurrentSkillActor))
  (Utilities|FlowControl|Sequence
    (:then_0
      (Utilities|IsValid _currentskillactor
        (:Is%20Valid
          (Actor|DestroyActor _currentskillactor))))
    (:then_1
      (Utilities|IsValid _currentweaponactor
        (:Is%20Valid
          (Actor|DestroyActor _currentweaponactor))))))

(fn ConstructionScript)

(fn OnRepWeaponIndex
  (Utilities|IsValid (Variables|Default|GetCurrentWeaponActor)
    (:Is%20Valid
      (Actor|DestroyActor (Variables|Default|GetCurrentWeaponActor)))
    (:Is%20Not%20Valid
      _))
  (bind _returnvalue (Game|SpawnActorfromClass (Utilities|Select :Index (Variables|Default|GetWeaponIndex) :NewEnumerator3 0 :NewEnumerator0 "/Game/BlackShield/Blueprints/Weapon/BP_WeaponGun.BP_WeaponGun_C" :NewEnumerator1 "/Game/BlackShield/Blueprints/Weapon/BP_FireGun.BP_FireGun_C") (Transformation|GetActorTransform) "Undefined" 0 0))
  (bind _asbp_weapon_base (Utilities|Casting|CastToBP_WeaponBase _returnvalue))
  (bind _output_get (Variables|Default|SetCurrentWeaponActor _asbp_weapon_base))
  (Variables|/Game/BlackShield/Blueprints/Weapon/BP_WeaponBase.BP_WeaponBase_C|SetCharacterActor _output_get (Variables|Default|GetCharacter))
  (Development|PrintString (Utilities|GetDisplayName _output_get) true true "(R=0.000000,G=0.660000,B=1.000000,A=1.000000)" 1e+01))

(fn OnRepSkillIndex
  (Utilities|IsValid (Variables|Default|GetCurrentSkillActor)
    (:Is%20Valid
      (Actor|DestroyActor (Variables|Default|GetCurrentSkillActor)))
    (:Is%20Not%20Valid
      _))
  (bind _returnvalue (Game|SpawnActorfromClass (Utilities|Select :Index (Variables|Default|GetSkillIndex) :NewEnumerator2 0 :NewEnumerator0 "/Game/StarVR/Blueprints/Hands/BP_Knife.BP_Knife_C" :NewEnumerator1 "/Game/StarVR/Blueprints/Teleport/BP_TeleportPoint_Advanced.BP_TeleportPoint_Advanced_C") (Transformation|GetActorTransform) "Undefined" 0 0))
  (bind _asbp_skill_base (Utilities|Casting|CastToBP_SkillBase _returnvalue))
  (bind _output_get (Variables|Default|SetCurrentSkillActor _asbp_skill_base))
  (Variables|/Game/StarVR/Blueprints/Teleport/BP_SkillBase.BP_SkillBase_C|SetChracterActor _output_get (Variables|Default|GetCharacter))
  (Development|PrintString (Utilities|GetDisplayName _output_get) true true "(R=0.000000,G=0.660000,B=1.000000,A=1.000000)" 1e+01))

(fn IsLocally
  (bind _character (Variables|Default|GetCharacter))
  (Utilities|IsValid _character
    (:Is%20Valid
      (return (Pawn|IsLocallyControlled _character)))
    (:Is%20Not%20Valid
      (return false))))

(fn CurSkillNeedUpdate
  (bind _currentskillactor (Variables|Default|GetCurrentSkillActor))
  (Utilities|IsValid _currentskillactor
    (:Is%20Valid
      (return (Default|IsNeedUpdate _currentskillactor)))
    (:Is%20Not%20Valid
      (return false))))