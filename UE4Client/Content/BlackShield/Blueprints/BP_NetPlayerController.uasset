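; BlackShield's networked player controller, covering match start, pawn spawning, ready state and damage feedback.
; GameStart swaps the lobby level for L_PVP, and SpawnPlayer possesses a new flying character at a random tagged PlayerStart or fallback point, also five seconds after death.
; A local BP_HurtHUDMgr shows hit damage.
; Outside active play, motion-controller traces click BPI_UI actors; test keys drive scoreboard, button and menu calls on the GameInstance.
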(event Custom|SetCharacterIndex
  (params (Index :type Integer))
  ;[1 1 1] SetCharacterIndex
  (CallFunction|SetCharacterIndexClient Index))

(event Custom|SetCharacterIndexClient
  (params (Index :type Integer))
  ;[1 1 1] SetCharacterIndex
  (bind _asbp_bschr_movement (Utilities|Casting|CastToBP_BSChrMovement (Pawn|GetControlledPawn)))
  (Default|SetCharacterIndex _asbp_bschr_movement Index))

(event Custom|PlayerDeathEvent
  ;[1 1 1] 死亡逻辑
  (Development|PrintString "PlayerDeathEvent")
  (Utilities|FlowControl|Delay 5.0)
  (CallFunction|SpawnPlayer))

(event Custom|PlayerReady
  (params (Ready :type Boolean))
  ;[1 1 1] 玩家准备消息发送
  (bind _asbp_player_state_net (Utilities|Casting|CastToBP_PlayerStateNet (Variables|GetPlayerState)))
  (Variables|/Game/BlackShield/Blueprints/Character/BP_PlayerStateNet.BP_PlayerStateNet_C|SetIsReadyForPlay _asbp_player_state_net Ready))

(event Custom|HitTargetEvent
  (params (HitActor :type Actor%20Object%20Reference) (HitDamage :type Integer))
  ;[1 1 1] 攻击目标的伤害提示
  (if (Pawn|IsLocalPlayerController)
    (bind _outactors (Actor|GetAllActorsOfClass "/Game/BlackShield/Blueprints/UI/PlayerGizmos/BP_HurtHUDMgr.BP_HurtHUDMgr_C"))
    (Default|DisplayHurt _outactors HitActor (Math|Float|Truncate (* HitDamage -1.0)) 5e+01)))

(event Custom|GameStart
  ;[1 1 1] 游戏开始逻辑
  (Utilities|FlowControl|Sequence
    (:then_0
      (Game|UnloadStreamLevel(byName) "L_MainLobby"))
    (:then_1
      (Game|LoadStreamLevel(byName) "L_PVP" true)
      (CallFunction|SpawnPlayer))))

(event Custom|SpawnPlayer
  (bind _returnvalue (Math|Vector|MakeVector 2e+03 2e+03 0.0))
  (bind _returnvalue_2 (Math|Vector|MakeVector 0.0 0.0 0.0))
  (bind _returnvalue_3 (Pawn|GetControlledPawn))
  (bind _playerstartspawned (Variables|Default|GetPlayerStartSpawned))
  (bind _returnvalue_4 (Utilities|Array|Length _playerstartspawned))
  (bind _returnvalue_5 (Math|Random|RandomPointinBoundingBox _returnvalue_2 _returnvalue))
  (bind _returnvalue_6 (<= _returnvalue_4 0))
  (bind _returnvalue_7 (- _returnvalue_4 1))
  (bind _returnvalue_8 (Math|Transform|MakeTransform _returnvalue_5))
  (bind _returnvalue_9 (Math|Random|RandomIntegerinRange 0 _returnvalue_7))
  (bind _item (Utilities|Array|Get(acopy) _playerstartspawned _returnvalue_9))
  (bind _returnvalue_10 (Transformation|GetActorTransform _item))
  (bind (_location _rotation) (Math|Transform|BreakTransform _returnvalue_10))
  (bind _returnvalue_11 (Math|Transform|MakeTransform _location _rotation))
  (bind _returnvalue_12 (select _returnvalue_6 _returnvalue_8 _returnvalue_11))
  ;[1 1 1] 服务器端上的各端角色生成
  (Development|PrintString "SpawnPlayerServer")
  (Utilities|IsValid _returnvalue_3
    (:Is%20Valid
      (Actor|DestroyActor _returnvalue_3))
    (:Is%20Not%20Valid
      _))
  (Utilities|Array|Clear (Variables|Default|GetPlayerStartSpawned))
  (bind _outactors (Actor|GetAllActorsOfClass "/Script/Engine.PlayerStart"))
  (for _array_element _outactors
    (if (Utilities|Name|Equal(Name) (Variables|/Script/Engine.PlayerStart|GetPlayerStartTag _array_element) "SpawnPlayer")
      (Utilities|Array|Add (Variables|Default|GetPlayerStartSpawned) _array_element)))
  (bind _returnvalue_13 (Game|SpawnActorfromClass "/Game/BlackShield/Blueprints/Character/BP_BSChrMovement_Fly.BP_BSChrMovement_Fly_C" _returnvalue_12 "AlwaysSpawn" 0 0))
  (Pawn|Possess _returnvalue_13)
  (Transformation|SetActorLocation _returnvalue_13 (.Location (Math|Transform|BreakTransform _returnvalue_12)) false true)
  (Default|SetBodyTransluncyClient _returnvalue_13))

(event EventBeginPlay
  ;[1 1 1] 目标伤害指示对象生成
  (if (Pawn|IsLocalController)
    (bind _returnvalue (Game|SpawnActorfromClass "/Game/BlackShield/Blueprints/UI/PlayerGizmos/BP_HurtHUDMgr.BP_HurtHUDMgr_C" (Transformation|GetActorTransform) "AlwaysSpawn" 0 0))
    (Variables|Default|SetHurtHudMgr _returnvalue)))

(event EventEndPlay
  (params (EndPlayReason :type EEndPlayReason%20Enum :default "Destroyed"))
  (bind _hurthudmgr (Variables|Default|GetHurtHudMgr))
  ;[1 1 1] Actor销毁附加功能处理
  (Utilities|IsValid _hurthudmgr
    (:Is%20Valid
      (Actor|DestroyActor _hurthudmgr))))

(event EventTick
  (params (DeltaSeconds :type Float%20%28single-precision%29))
  (bind _returnvalue (Game|GetPlayerCameraManager 0))
  (bind _currenthand (Variables|Default|GetCurrentHand))
  (bind _returnvalue_2 (Transformation|GetActorLocation _returnvalue))
  (bind (_outposition _outorientation) (Class|SteamVRFunctionLibrary|GetHandPositionandOrientation 0 _currenthand))
  ;[0 0.9341 1] 测试代码
  ;;[1 1 1] 手柄按钮测试代码
  (bind _asbp_net_game_state (Utilities|Casting|CastToBP_NetGameState (Game|GetGameState))
    (:then
      (if (not (Variables|/Game/BlackShield/Blueprints/BP_NetGameState.BP_NetGameState_C|GetGamePlaying _asbp_net_game_state))
        (Collision|LineTraceByChannel (+ _returnvalue_2 _outposition) (+ _returnvalue_2 (Math|Vector|RotateVector "5000.000000, 0, 0" _outorientation)) "TraceTypeQuery3" true 0 "ForOneFrame" :!label _label)))
    (:CastFailed
      (goto _label))))

(event Input|ActionEvents|InputActionFire
  (params (Key :type Key%20Structure :default "AnyKey"))
  (bind _returnvalue (Game|GetPlayerCameraManager 0))
  (bind _returnvalue_2 (Transformation|GetActorLocation _returnvalue))
  ;[0 0.9341 1] 测试代码
  ;;[1 1 1] 手柄按钮测试代码
  (:Pressed
    (bind _asbp_net_game_state (Utilities|Casting|CastToBP_NetGameState (Game|GetGameState))
      (:then
        (if (not (Variables|/Game/BlackShield/Blueprints/BP_NetGameState.BP_NetGameState_C|GetGamePlaying _asbp_net_game_state))
          (Variables|Default|SetCurrentHand "Right" :!label _label)
          (bind _outhit (Collision|LineTraceByChannel (+ _returnvalue_2 (.OutPosition (Class|SteamVRFunctionLibrary|GetHandPositionandOrientation 0 (Variables|Default|GetCurrentHand)))) (+ _returnvalue_2 (Math|Vector|RotateVector "5000.000000, 0, 0" (.OutOrientation (Class|SteamVRFunctionLibrary|GetHandPositionandOrientation 0 (Variables|Default|GetCurrentHand))))) "TraceTypeQuery3" true 0 "None"))
          (if (Utilities|DoesObjectImplementInterface (.HitActor (Collision|BreakHitResult _outhit)) "/Game/BlackShield/Blueprints/UI/BPI_UI.BPI_UI_C")
            (Class|BPIUI|OnClickButton(Message) (.HitActor (Collision|BreakHitResult _outhit))))))
      (:CastFailed
        (goto _label)))))

(event Input|KeyboardEvents|Tab
  (params (Key :type Key%20Structure :default "AnyKey"))
  ;[0 0.9341 1] 测试代码
  ;;[1 1 1] 积分板测试显示
  (:Pressed
    (bind _asbp_net_game_instance (Utilities|Casting|CastToBP_NetGameInstance (Game|GetGameInstance)))
    (Default|ShowScoreBoard _asbp_net_game_instance true))
  (:Released
    (bind _asbp_net_game_instance_2 (Utilities|Casting|CastToBP_NetGameInstance (Game|GetGameInstance)))
    (Default|ShowScoreBoard _asbp_net_game_instance_2 false)))

(event Input|KeyboardEvents|L
  (params (Key :type Key%20Structure :default "AnyKey"))
  ;[0 0.9341 1] 测试代码
  ;;[1 1 1] 退出到主菜单测试
  (:Pressed
    (bind _asbp_net_game_instance (Utilities|Casting|CastToBP_NetGameInstance (Game|GetGameInstance)))
    (Default|ReturntoMainMenu _asbp_net_game_instance)))

(event Input|MouseEvents|LeftMouseButton
  (params (Key :type Key%20Structure :default "AnyKey"))
  ;[0 0.9341 1] 测试代码
  ;;[1 1 1] 按钮模拟测试代码
  (:Pressed
    (bind _asbp_net_game_instance (Utilities|Casting|CastToBP_NetGameInstance (Game|GetGameInstance)))
    (Default|ButtonDown _asbp_net_game_instance)))

(fn ConstructionScript)