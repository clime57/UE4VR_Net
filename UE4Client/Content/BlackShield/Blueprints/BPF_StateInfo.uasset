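; Blueprint function library with one check, StartPlayingCondition, that reports whether play can start as one of three enum states.
; It returns the first state when the GameState's PlayerArray holds fewer than the required minimum.
; Otherwise it scans that array, returning the third state at the first entry that is the passed Player or a BP_PlayerStateNet flagged IsReadyForPlay.
; The second state results when the scan finds neither.
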(fn StartPlayingCondition
  (params (Player :type Player%20State%20Object%20Reference) (MinPlayer :type Integer))
  (bind _returnvalue (Game|GetGameState Player))
  (bind _playerarray (Variables|/Script/Engine.GameState|GetPlayerArray _returnvalue))
  (if (< (Utilities|Array|Length _playerarray) MinPlayer)
    (return "NewEnumerator0")
    (else
      (bind _array_element (Utilities|Array|ForEachLoopwithBreak _playerarray)
        (:LoopBody
          (if (!= Player _array_element)
            (bind _asbp_player_state_net (Utilities|Casting|CastToBP_PlayerStateNet _array_element))
            (if (Variables|/Game/BlackShield/Blueprints/Character/BP_PlayerStateNet.BP_PlayerStateNet_C|GetIsReadyForPlay _asbp_player_state_net)
              (return "NewEnumerator2"))
            (else
              (return "NewEnumerator2"))))
        (:Completed
          (return "NewEnumerator1"))))))