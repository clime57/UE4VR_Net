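; Networked game mode that holds joining players in a waiting phase until the match starts.
; On login it flags the host, notifies BP_NetGameState, then starts late joiners immediately or indexes waiting players by matching "Player{N}" PlayerStart tags.
; Waiting players start at the "FreeView" start; waiting-pawn spawn and possession nodes are disconnected.
; StartGame sets GamePlaying and starts every controller; a test event randomizes player board data.
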(event Custom|TestForPlayerScore
  (Networking|SwitchHasAuthority
    (:Authority
      (for _array_element (Variables|/Script/Engine.GameState|GetPlayerArray (Game|GetGameState))
        (bind _asbp_player_state_net (Utilities|Casting|CastToBP_PlayerStateNet _array_element))
        (Default|RandomBoardData _asbp_player_state_net)))))

(event Custom|StartGame
  (Networking|SwitchHasAuthority
    (:Authority
      (bind _asbp_net_game_state (Utilities|Casting|CastToBP_NetGameState (Game|GetGameState)))
      (Variables|/Game/BlackShield/Blueprints/BP_NetGameState.BP_NetGameState_C|SetGamePlaying _asbp_net_game_state true)
      (bind _outactors (Actor|GetAllActorsOfClass "/Game/BlackShield/Blueprints/BP_NetPlayerController.BP_NetPlayerController_C"))
      (Default|GameStart _outactors))))

(event EventPostLogin
  (params (NewPlayer :type Player%20Controller%20Object%20Reference))
  (bind _returnvalue (Game|GetGameState))
  (bind _returnvalue_2 (Game|GetPlayerController 0))
  (bind _playerarray (Variables|/Script/Engine.GameState|GetPlayerArray _returnvalue))
  (bind _returnvalue_3 (Utilities|Array|Length _playerarray))
  (Networking|SwitchHasAuthority
    (:Authority
      (if (== _returnvalue_2 NewPlayer)
        (bind _asbp_player_state_net (Utilities|Casting|CastToBP_PlayerStateNet (Variables|/Script/Engine.Controller|GetPlayerState _returnvalue_2)))
        (Variables|/Game/BlackShield/Blueprints/Character/BP_PlayerStateNet.BP_PlayerStateNet_C|SetIsHostPlayer _asbp_player_state_net true))
      (bind _asbp_net_game_state (Utilities|Casting|CastToBP_NetGameState (Game|GetGameState)))
      (Default|PlayerLogin _asbp_net_game_state NewPlayer)
      (if (Variables|Default|GetReadyStartMatch)
        ;[1 1 1] 已经开始游戏直接开始
        (bind _asbp_net_player_controller (Utilities|Casting|CastToBP_NetPlayerController NewPlayer))
        (Default|GameStart _asbp_net_player_controller)
        (else
          ;[1 1 1] 没有开始比赛时等待其他玩家
          (Variables|Default|SetPlayerSpawnStart 0)
          (bind _outactors (Actor|GetAllActorsOfClass "/Script/Engine.PlayerStart"))
          (bind _array_element (Utilities|Array|ForEachLoopwithBreak _outactors)
            (:LoopBody
              (if (Utilities|Name|Equal(Name) (Variables|/Script/Engine.PlayerStart|GetPlayerStartTag _array_element) (Utilities|String|StringToName (Utilities|String|ToString(Text) (Utilities|Text|FormatText "Player{ID}" (Utilities|Text|ToText(Integer) _returnvalue_3)))))
                (Variables|Default|SetPlayerSpawnStart _array_element)))
            (:Completed
              (Utilities|IsValid (Variables|Default|GetPlayerSpawnStart)
                (:Is%20Valid
                  (bind _asbp_player_state_net_2 (Utilities|Casting|CastToBP_PlayerStateNet (Variables|/Script/Engine.Controller|GetPlayerState NewPlayer)))
                  (Variables|/Game/BlackShield/Blueprints/Character/BP_PlayerStateNet.BP_PlayerStateNet_C|SetPlayerIndex _asbp_player_state_net_2 _returnvalue_3))))))))))

(event EventOnLogout
  (params (ExitingController :type Controller%20Object%20Reference))
  (bind _asplayer_controller (Utilities|Casting|CastToPlayerController ExitingController))
  (bind _asbp_net_game_state (Utilities|Casting|CastToBP_NetGameState (Game|GetGameState)))
  (Default|PlayerLogout _asbp_net_game_state _asplayer_controller))

(fn ConstructionScript)

(fn ReadytoStartMatch
  (return (Variables|Default|GetReadyStartMatch)))

(fn ChoosePlayerStart
  (params (Player :type Controller%20Object%20Reference))
  (if (Variables|Default|GetReadyStartMatch)
    (return 0)
    (else
      (bind _outactors (Actor|GetAllActorsOfClass "/Script/Engine.PlayerStart"))
      (bind _array_element (Utilities|Array|ForEachLoopwithBreak _outactors :!label _label)
        (:LoopBody
          (if (Utilities|Name|Equal(Name) (Variables|/Script/Engine.PlayerStart|GetPlayerStartTag _array_element) "FreeView")
            (LocalVariables|SetFreePlayerStart _array_element)
            (goto _label Break)))
        (:Completed
          (return (LocalVariables|GetFreePlayerStart)))))))